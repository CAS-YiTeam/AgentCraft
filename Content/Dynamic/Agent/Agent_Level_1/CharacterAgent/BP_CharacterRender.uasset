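; Character render Blueprint that builds a layered, outlined character with SDF face shading from a RenderPack.
; Construction assigns skeletal meshes, creates dynamic outline and face materials, and makes the outline, hair and eye components follow the base mesh's pose.
; It passes the face material and light to BPCSDF for the SDF update.
; M_Mask material swaps split hair and eyes onto separate PostHair and PostEye mesh copies.
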(event Custom|cacl_sdf
  (Variables|Character|GetMesh
    (:then
      (Default|Update (Variables|Default|GetBPC_SDF) (Variables|Character|GetMesh) (Variables|Default|GetSingle%20Player?) (Variables|Default|GetFace_sdf_Inst) (Variables|Default|GetSDF_OffSet) (Variables|Default|GetLight) 0.02 "頭"))
    (:else)))

(event EventBeginPlay)

(event Collision|EventActorBeginOverlap
  (params (OtherActor :type Actor%20Object%20Reference)))

(event EventTick
  (params (DeltaSeconds :type Float%20%28single-precision%29)))

(fn ConstructionScript
  (Utilities|FlowControl|Sequence
    (:then_0
      (CallFunction|SetMesh))
    (:then_1
      (CallFunction|CaclSdf))
    (:then_2
      (CallFunction|SetHairEyeMask))))

(fn SetMesh
  (bind _renderpack (Variables|Data|GetRenderPack)
    (:then
      (Utilities|FlowControl|Sequence
        (:then_0
          (bind _basemesh (Variables|/Game/Static/BluePrints/SubBlueprints/BP_Dataasset.BP_Dataasset_C|GetBasemesh _renderpack)
            (:then
              (Components|SkeletalMesh|SetSkeletalMeshAsset (Variables|Character|GetMesh) _basemesh)
              (Variables|/Script/Engine.SkeletalMeshComponent|SetSkeletalMeshAsset (Variables|Default|GetOutLine) (Variables|/Game/Static/BluePrints/SubBlueprints/BP_Dataasset.BP_Dataasset_C|GetOutLinemesh _renderpack))
              (for (_array_element _array_index) (Variables|/Game/Static/BluePrints/SubBlueprints/BP_Dataasset.BP_Dataasset_C|GetOutLineMaterials (Variables|Data|GetRenderPack))
                (bind _asmaterial_instance_constant (Utilities|Casting|CastToMaterialInstanceConstant _array_element))
                (bind _returnvalue (Rendering|Material|CreateDynamicMaterialInstance "/IM4U/Material/MaterialTool/M_OutLine_Inst.M_OutLine_Inst" "None" "None" :!class /Script/Engine.KismetMaterialLibrary))
                (bind _output_get (LocalVariables|SetMaterialsDynamic _returnvalue))
                (bind _returnvalue_2 (Rendering|Material|GetVectorParameterValue _asmaterial_instance_constant "OutLineColor" :!class /Script/Engine.MaterialInstanceConstant))
                (bind _returnvalue_3 (Rendering|Material|GetScalarParameterValue _asmaterial_instance_constant "OutLineSize" :!class /Script/Engine.MaterialInstanceConstant))
                (Utilities|FlowControl|Sequence
                  (:then_0
                    (Rendering|Material|SetScalarParameterValue _returnvalue "OutLineSize" _returnvalue_3 :!class /Script/Engine.MaterialInstanceDynamic))
                  (:then_1
                    (Rendering|Material|SetVectorParameterValue _returnvalue "OutLineColor" _returnvalue_2 :!class /Script/Engine.MaterialInstanceDynamic)))
                (Rendering|Material|SetMaterial (Variables|Default|GetOutLine) _array_index _output_get)))
            (:else)))
        (:then_1
          (bind (_array_element_2 _array_index_2) (Utilities|Array|ForEachLoopwithBreak (Variables|/Game/Static/BluePrints/SubBlueprints/BP_Dataasset.BP_Dataasset_C|GetBaseMaterials _renderpack) :!label _label)
            (:LoopBody
              (if (== _array_element_2 (Variables|/Game/Static/BluePrints/SubBlueprints/BP_Dataasset.BP_Dataasset_C|GetFaceMaterial _renderpack))
                (goto _label Break)))
            (:Completed
              (bind _returnvalue_4 (Rendering|Material|CreateDynamicMaterialInstance (Variables|Character|GetMesh) _array_index_2 0 "" :!class /Script/Engine.PrimitiveComponent))
              (Variables|Default|SetFace_sdf_Inst _returnvalue_4))))
        (:then_2
          (Components|SkinnedMesh|SetLeaderPoseComponent (Variables|Default|GetPost_Eye) (Variables|Character|GetMesh) false false))))
    (:else)))

(fn SetHairEyeMask
  (bind _renderpack (Variables|Data|GetRenderPack))
  (bind _basematerials (Variables|/Game/Static/BluePrints/SubBlueprints/BP_Dataasset.BP_Dataasset_C|GetBaseMaterials _renderpack))
  (Utilities|FlowControl|Sequence
    (:then_0
      (bind _hairmaterial (Variables|/Game/Static/BluePrints/SubBlueprints/BP_Dataasset.BP_Dataasset_C|GetHairMaterial _renderpack)
        (:then
          (for (_array_element _array_index) _basematerials
            (if (== _array_element _hairmaterial)
              (Rendering|Material|SetMaterial (Variables|Character|GetMesh) _array_index "/IM4U/Material/MaterialTool/Master/M_Mask.M_Mask")
              (else
                (Rendering|Material|SetMaterial (Variables|Default|GetPost_Hair) _array_index "/IM4U/Material/MaterialTool/Master/M_Mask.M_Mask"))))
          (bind _eyematerial (Variables|/Game/Static/BluePrints/SubBlueprints/BP_Dataasset.BP_Dataasset_C|GetEyeMaterial (Variables|Data|GetRenderPack))
            (:then
              (for (_array_element_2 _array_index_2) _basematerials
                (if (== _array_element_2 _eyematerial)
                  (Rendering|Material|SetMaterial (Variables|Character|GetMesh) _array_index_2 "/IM4U/Material/MaterialTool/Master/M_Mask.M_Mask")
                  (else
                    (Rendering|Material|SetMaterial (Variables|Default|GetPost_Eye) _array_index_2 "/IM4U/Material/MaterialTool/Master/M_Mask.M_Mask")))))
            (:else)))
        (:else)))))